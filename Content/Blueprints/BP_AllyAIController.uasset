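; AI controller for allies that plays attack and failed-attack animations on its controlled BaseCharacter pawn.
; Attack plays the montage supplied by the character, while FailAttack stops the current montage and plays the character's flinch montage instead.
; Both events call CompleteAttack only when their montage completes, with no handling for interruption.
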(event EventBeginPlay)

(event EventTick
  (params (DeltaSeconds :type Float%20%28single-precision%29)))

(event EventAttack
  (bind _asbase_character (Utilities|Casting|CastToBaseCharacter (Pawn|GetControlledPawn)))
  (bind _returnvalue (Class|BaseCharacter|GetAttackAnimation _asbase_character))
  (Animation|Montage|PlayMontage (Variables|/Script/Engine.Character|GetMesh _asbase_character) _returnvalue
    (:OnCompleted
      (Class|CombatAIController|CompleteAttack))))

(event EventFailAttack
  (bind _asbase_character (Utilities|Casting|CastToBaseCharacter (Pawn|GetControlledPawn)))
  (Animation|StopAnimMontage _asbase_character 0)
  (bind _returnvalue (Class|BaseCharacter|GetFlinchAnimation _asbase_character))
  (Animation|Montage|PlayMontage (Variables|/Script/Engine.Character|GetMesh _asbase_character) _returnvalue
    (:OnCompleted
      (Class|CombatAIController|CompleteAttack))))

(fn ConstructionScript)